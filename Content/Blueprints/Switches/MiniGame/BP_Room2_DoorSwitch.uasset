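; BP_Room2_DoorSwitch is a minigame switch that swings its linked door open and closed.
; The IsToggled RepNotify rotates DoorToOpen 90 degrees about local Z, reverses the stored rotation when untoggled, and swaps the switch mesh material between green and red.
; Once InitFinished is set, each change also plays a click at the switch and a creak at the door.
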(event EventBeginPlay)

(event Collision|EventActorBeginOverlap
  (params (OtherActor :type Actor%20Object%20Reference)))

(event EventTick
  (params (DeltaSeconds :type Float%20%28single-precision%29)))

(event EventOnRepIsToggled
  (bind _doortoopen (Variables|Default|GetDoorToOpen))
  (if (Variables|Default|GetbIsToggled)
    (bind _output_get (Variables|Default|SetLocalZRotation "0,90.000000, 0"))
    (Transformation|AddActorLocalRotation _doortoopen _output_get false false)
    (Rendering|Material|SetMaterial (Variables|Default|GetStaticMeshComponent) 0 "/Game/Materials/Green.Green")
    (else
      (Transformation|AddActorLocalRotation _doortoopen (* (Variables|Default|GetLocalZRotation) -1) false false)
      (Variables|Default|SetLocalZRotation "0, 0, 0")
      (Rendering|Material|SetMaterial (Variables|Default|GetStaticMeshComponent) 0 "/Game/Materials/Red.Red")))
  (if (Variables|Default|GetbInitFinished)
    (Audio|PlaySoundatLocation "/Game/Audio/LightSwitch03_Cue.LightSwitch03_Cue" (Transformation|GetActorLocation) "0, 0, 0" 1.0 1.0 0.0 0 0 0)
    (Audio|PlaySoundatLocation "/Game/Audio/WoodenCreak.WoodenCreak" (Transformation|GetActorLocation (Variables|Default|GetDoorToOpen)) "0, 0, 0" 1.0 1.0 0.0 0 0 0)))

(fn ConstructionScript)