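; BP_Room1LightSwitch is a mini-game light switch that reveals or hides a text actor and another switch actor.
; It extends a parent switch, calling the parent's IsToggled RepNotify before applying its own changes.
; When toggled on, it shows the text and unhides the switch with query and physics collision.
; When off, it hides both and disables the switch's collision.
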(event EventBeginPlay)

(event Collision|EventActorBeginOverlap
  (params (OtherActor :type Actor%20Object%20Reference)))

(event EventTick
  (params (DeltaSeconds :type Float%20%28single-precision%29)))

(event EventOnRepIsToggled
  (bind _textactor (Variables|Default|GetTextActor))
  (bind _switchactor (Variables|Default|GetSwitchActor))
  (bind _textrender (Variables|/Script/Engine.TextRenderActor|GetTextRender _textactor))
  (bind _staticmeshcomponent (Variables|/Script/TF.TFInteractable|GetStaticMeshComponent _switchactor))
  (|CallParentFunction)
  (if (Variables|Default|GetbIsToggled)
    (Rendering|SetVisibility _textrender true true)
    (Rendering|SetActorHiddenInGame _switchactor false)
    (Collision|SetCollisionEnabled _staticmeshcomponent "QueryAndPhysics")
    (else
      (Rendering|SetVisibility _textrender false false)
      (Rendering|SetActorHiddenInGame _switchactor true)
      (Collision|SetCollisionEnabled _staticmeshcomponent "NoCollision"))))

(fn ConstructionScript)