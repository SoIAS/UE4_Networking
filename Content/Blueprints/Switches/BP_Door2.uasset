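; BP_Door2 is a replicated interactable door that swings open and closed as it is toggled.
; The IsToggled rep-notify applies a 90-degree local rotation on opening and reverses the stored rotation on closing, guarding against repeated opening.
; A multicast used event plays a wooden creak at the door's location, and the tooltip combines Open or Close with the door's name.
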(event EventBeginPlay)

(event Collision|EventActorBeginOverlap
  (params (OtherActor :type Actor%20Object%20Reference)))

(event EventTick
  (params (DeltaSeconds :type Float%20%28single-precision%29)))

(event EventOnRepIsToggled
  (if (Variables|Default|GetbIsToggled)
    (if (not (Math|Rotator|Equal(Rotator) (Variables|Default|GetLocalZRotation) "0.000000,90.000000, 0" 0.0001))
      (bind _output_get (Variables|Default|SetLocalZRotation "0,90.000000, 0"))
      (Transformation|AddActorLocalRotation _output_get false false))
    (else
      (Transformation|AddActorLocalRotation (* (Variables|Default|GetLocalZRotation) -1) false false)
      (Variables|Default|SetLocalZRotation "0, 0, 0"))))

(event EventBlueprintNetMulticastonUsed
  (if true
    (Audio|PlaySoundatLocation "/Game/Audio/WoodenCreak.WoodenCreak" (Transformation|GetActorLocation) "0, 0, 0" 1.0 1.0 0.0 0 0 0)))

(fn ConstructionScript)

(fn GetInteractableTooltipText
  (if (Variables|Default|GetbIsToggled)
    (LocalVariables|SetActionString "Close ")
    (else
      (LocalVariables|SetActionString "Open ")))
  (return (Utilities|String|Append (LocalVariables|GetActionString) (Utilities|String|ToString(Name) (Variables|Default|GetName)))))