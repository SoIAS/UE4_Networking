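; Player controller that creates the local player's HUD widgets: interaction tooltip, inventory and main UI.
; On BeginPlay it waits briefly, then calls one creation function per widget in sequence.
; Each function checks that the controller is local, creates the widget with itself as owning player, stores the reference and adds it to the viewport.
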(event EventBeginPlay
  (Utilities|FlowControl|Delay 0.1)
  (CallFunction|CreateInteractionTooltipWidget)
  (CallFunction|CreateInventoryWidget)
  (CallFunction|CreateMainUIWidget))

(event EventTick
  (params (DeltaSeconds :type Float%20%28single-precision%29)))

(fn ConstructionScript)

(fn CreateInteractionTooltipWidget
  (if (Pawn|IsLocalController)
    (bind _returnvalue (UserInterface|CreateWidget "/Game/Widgets/InteractableTooltip.InteractableTooltip_C" self))
    (bind _output_get (Variables|Default|SetInteractableTooltip _returnvalue))
    (UserInterface|Viewport|AddtoViewport _output_get 0)))

(fn CreateInventoryWidget
  (if (Pawn|IsLocalController)
    (bind _returnvalue (UserInterface|CreateWidget "/Game/Widgets/InventoryWidget.InventoryWidget_C" self))
    (bind _output_get (Variables|Default|SetInventoryWidget _returnvalue))
    (UserInterface|Viewport|AddtoViewport _output_get 0)))

(fn CreateMainUIWidget
  (if (Pawn|IsLocalController)
    (bind _returnvalue (UserInterface|CreateWidget "/Game/Widgets/MainUI.MainUI_C" self))
    (bind _output_get (Variables|Default|SetMainUIWidget _returnvalue))
    (UserInterface|Viewport|AddtoViewport _output_get 0)))